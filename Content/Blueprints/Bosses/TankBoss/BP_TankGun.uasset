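; BP_TankGun is the twin-gun turret of the tank boss, firing while the player is inside its trigger box.
; Box overlap starts a looping one-second timer and an immediate Shoot, which is skipped while BP_TheTank reports death or menu.
; Each gun line-traces within a random narrow cone, messages the hit actor, and plays muzzle effects, plus ricochet sounds for non-player hits.
; Tick disables both gun meshes' collision once the boss dies.
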(event OnComponentBeginOverlap(Box)
  (params (OverlappedComponent :type Primitive%20Component%20Object%20Reference) (OtherActor :type Actor%20Object%20Reference) (OtherComp :type Primitive%20Component%20Object%20Reference) (OtherBodyIndex :type Integer) (bFromSweep :type Boolean) (SweepResult :type Hit%20Result%20Structure%20%28by%20ref%29))
  (if (== OtherActor (Game|GetPlayerCharacter 0))
    (bind _output_get (Variables|Default|SetPlayerInRange true))
    (Development|PrintString (Utilities|String|ToString(Boolean) _output_get))
    (bind _returnvalue (Utilities|Time|SetTimerbyEvent (EventDispatchers|CreateEvent :!event Custom|Shoot) 1.0 true))
    (Variables|Default|SetTimerRef _returnvalue)
    (CallFunction|Shoot)))

(event OnComponentEndOverlap(Box)
  (params (OverlappedComponent :type Primitive%20Component%20Object%20Reference) (OtherActor :type Actor%20Object%20Reference) (OtherComp :type Primitive%20Component%20Object%20Reference) (OtherBodyIndex :type Integer))
  (if (== OtherActor (Game|GetPlayerCharacter 0))
    (Variables|Default|SetPlayerInRange false)
    (Utilities|Time|ClearandInvalidateTimerbyHandle (Variables|Default|GetTimerRef))))

(event Custom|Shoot
  (bind _tankref (Variables|Default|GetTankRef))
  (if (not (or (Variables|/Game/Blueprints/Bosses/TankBoss/BP_TheTank.BP_TheTank_C|GetBossDead _tankref) (Variables|/Game/Blueprints/Bosses/TankBoss/BP_TheTank.BP_TheTank_C|GetMenu _tankref)))
    (Development|PrintString "Shooting" true true "(R=0.000000,G=0.660000,B=1.000000,A=1.000000)" 2.0 "Shooting")
    (Utilities|FlowControl|Sequence
      (:then_0
        (CallFunction|ShootGun (Variables|Default|GetTurretLShootDir) (Variables|Default|GetSM_TankGunL))
        (CallFunction|ShootGun (Variables|Default|GetTurretRShootDir) (Variables|Default|GetSM_TankGunR) 1)))))

(event EventBeginPlay
  (bind _returnvalue (Actor|GetActorOfClass "/Game/Blueprints/Bosses/TankBoss/BP_TheTank.BP_TheTank_C"))
  (Variables|Default|SetTankRef _returnvalue))

(event Collision|EventActorBeginOverlap
  (params (OtherActor :type Actor%20Object%20Reference)))

(event EventTick
  (params (DeltaSeconds :type Float%20%28single-precision%29))
  (if (Variables|/Game/Blueprints/Bosses/TankBoss/BP_TheTank.BP_TheTank_C|GetBossDead (Variables|Default|GetTankRef))
    (Collision|SetCollisionEnabled (Variables|Default|GetSM_TankGunL) "NoCollision")
    (Collision|SetCollisionEnabled (Variables|Default|GetSM_TankGunR) "NoCollision")))

(fn ConstructionScript)

(fn ShootGun
  (params (Shot%20Origin :type Arrow%20Component%20Object%20Reference) (Turret :type Skeletal%20Mesh%20Component%20Object%20Reference) (Index :type Integer))
  (bind _returnvalue (Utilities|Select :Index Index :Option%200 "MFlashL" :Option%201 "MFlashR"))
  (bind _returnvalue_2 (Transformation|GetSocketLocation Turret _returnvalue))
  (bind (_returnvalue_3 _returnvalue2) (|GetsTransformValuesforLineTrace_2 5e+03 Shot%20Origin)
    (:execute
      (Utilities|FlowControl|Sequence
        (:then_0
          (bind _outhit (Collision|LineTraceForObjects _returnvalue_3 _returnvalue2 (Variables|Default|GetObject%20Types) false 0 "ForDuration"))
          (Class|IShot|OnShot(Message) (.hitactor _outhit) 0 (.location _outhit))
          (if (!= (.hitactor _outhit) (Game|GetPlayerCharacter 0))
            (Audio|PlaySoundatLocation "/Game/Sound/Ricochet/SC_Ricochet.SC_Ricochet" (.location _outhit) "0, 0, 0" 5.0 1.0 0.0 "/Game/Sound/Ricochet/SA_Riccochet.SA_Riccochet" 0 0 0)))
        (:then_1
          (Effects|SpawnEmitteratLocation "/Game/StarterContent/Particles/P_Explosion.P_Explosion" _returnvalue_2 (Transformation|GetWorldRotation Turret))
          (Audio|SpawnSoundatLocation "/Game/Sound/BossSound/TankShot.TankShot" _returnvalue_2 "0, 0, 0" 0.3 1.0 0.0 "/Game/Sound/BossSound/SA_Tank.SA_Tank" 0))))))