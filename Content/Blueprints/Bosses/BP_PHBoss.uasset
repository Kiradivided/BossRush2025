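; BP_PHBoss is a shootable boss whose core is guarded by a breakable chest panel.
; On BeginPlay it snaps the panel mesh to the body's BodySocket.
; When OnShot reports a core hit while the panel is active, the panel explodes, detaches and is thrown off with physics.
; A core hit with the panel inactive spawns an explosion and destroys the boss.
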(event EventBeginPlay
  (Transformation|AttachComponentToComponent (Variables|Default|GetPanel) (Variables|Character|GetMesh) "BodySocket" "SnapToTarget" "SnapToTarget" "SnapToTarget" true)
  (Components|StaticMesh|SetStaticMesh (Variables|Default|GetPanel) "/Game/Objects/Bosses/PlaceHolder/BossChestPanel.BossChestPanel"))

(event Collision|EventActorBeginOverlap
  (params (OtherActor :type Actor%20Object%20Reference)))

(event EventTick
  (params (DeltaSeconds :type Float%20%28single-precision%29)))

(event EventOnShot
  (params (ComponentInput :type Actor%20Component%20Object%20Reference))
  (bind _returnvalue (Transformation|GetActorTransform))
  (bind _panel (Variables|Default|GetPanel))
  (bind _panel_2 (Variables|Default|GetPanel))
  (bind _returnvalue_2 (Transformation|GetWorldTransform _panel_2))
  (if (== ComponentInput (Variables|Default|GetCoreC))
    (if (Variables|Default|GetPanelActive)
      (Effects|SpawnEmitteratLocation "/Game/StarterContent/Particles/P_Explosion.P_Explosion" (.location _returnvalue_2) (.rotation _returnvalue_2) (.scale _returnvalue_2))
      (Transformation|DetachFromComponent (Variables|Default|GetPanel) "KeepRelative" "KeepRelative" "KeepRelative" true)
      (Physics|SetSimulatePhysics _panel true)
      (Physics|AddForce _panel (+ (Math|Vector|NegateVector (Math|Vector|GetUpVector _panel)) 1.2e+04) "None" true)
      (Variables|Default|SetPanelActive false)
      (else
        (Effects|SpawnEmitteratLocation "/Game/StarterContent/Particles/P_Explosion.P_Explosion" (.location _returnvalue) (.rotation _returnvalue) (.scale _returnvalue))
        (Actor|DestroyActor)))))

(fn ConstructionScript)