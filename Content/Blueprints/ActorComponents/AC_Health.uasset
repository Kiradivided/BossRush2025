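; AC_Health is an actor component that tracks a clamped health value for its owner.
; TakeDamage subtracts the damage and fires OnDamageTaken, then OnDeath whenever health is at zero.
; Heal adds a fixed amount, ignoring its HealthRestored input, and fires OnHeal.
; BeginPlay and Tick are unused, so all changes come through these two functions.
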(event EventBeginPlay)

(event EventTick
  (params (DeltaSeconds :type Float%20%28single-precision%29)))

(fn TakeDamage
  (params (Damage :type Float%20%28double-precision%29))
  (bind _output_get (Variables|Default|SetHealth (Math|Float|Clamp(Float) (- (Variables|Default|GetHealth) Damage) 0.0 (Variables|Default|GetMaxHealth))))
  (Default|CallOnDamageTaken)
  (if (<= _output_get 0.0)
    (Default|CallOnDeath)))

(fn Heal
  (params (HealthRestored :type Float%20%28double-precision%29))
  (Variables|Default|SetHealth (Math|Float|Clamp(Float) (+ (Variables|Default|GetHealth) 2e+01) 0.0 (Variables|Default|GetMaxHealth)))
  (Default|CallOnHeal))