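; First-person player character with Enhanced Input movement, look and jump, a revolver attached to the arms mesh, and a main HUD widget.
; Shooting plays montages, spends ammo and line-traces from a camera-based spread cone, calling OnShot on a hit boss; delays gate firing and reloading.
; Aiming zeroes the cone, as does the optional laser attachment at BeginPlay.
; A Health component prints changes and death, with debug damage and heal keys.
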(event OnDamageTaken(Health)
  ;[0.15 0.15 0.15 0.5] Prints Health on Changed
  (Development|PrintString (Utilities|String|ToString(Float) (Variables|/Game/Blueprints/ActorComponents/AC_Health.AC_Health_C|GetHealth (Variables|Default|GetHealth)))))

(event OnDeath(Health)
  ;[0.15 0.15 0.15 0.5] Get Good
  (Development|PrintString "You Died!" true true "(R=1.000000,G=0.121763,B=0.000000,A=1.000000)"))

(event OnHeal(Health)
  ;[0.15 0.15 0.15 0.5] Prints Health on Changed
  (Development|PrintString (Utilities|String|ToString(Float) (Variables|/Game/Blueprints/ActorComponents/AC_Health.AC_Health_C|GetHealth (Variables|Default|GetHealth)))))

(event Input|EnhancedActionEvents|EnhancedInputActionIA_ShootGun
  (params (ActionValue :type Boolean) (ElapsedSeconds :type Float%20%28double-precision%29) (TriggeredSeconds :type Float%20%28double-precision%29) (InputAction :type Input%20Action%20Object%20Reference :default "/Game/Blueprints/Player/Input/Actions/IA_ShootGun.IA_ShootGun"))
  (bind (_returnvalue _returnvalue2) (|GetsTransformValuesforLineTrace 5e+03))
  (Development|PrintString (Utilities|String|ToString(Integer) (Variables|Default|GetBCount)))
  (if (> (Variables|Default|GetBCount) 0)
    (if (Variables|Default|GetCanFire)
      (Variables|Default|SetCanFire false)
      (Animation|Montage|PlayMontage (Variables|Default|GetFutureArmsMaybe) "/Game/Blueprints/Player/Animations/PH/PHFire_Montage.PHFire_Montage"
        (:then
          (Components|Animation|PlayAnimation (Variables|Default|Getgun) "/Game/Objects/Guns/RevolverLukaFinal/Animations/Revolver_Final_Justyn_TestAnim.Revolver_Final_Justyn_TestAnim" false)
          (bind _result (Math|Integer|DecrementInt (Variables|Default|GetBCount))
            (:%20%20
              (Variables|Default|SetBCount _result)
              (Utilities|FlowControl|Sequence
                (:then_0
                  ;[0.15 0.15 0.15 0.5] Creates a Single Line Trace - Basically Hit Scan
                  (bind _outhit (Collision|LineTraceForObjects _returnvalue _returnvalue2 (Variables|Default|GetObject%20Types) false 0 "Persistent"))
                  ;[0.15 0.15 0.15 0.5] If true it will cast to the boss bp which then calls the interface On shot
                  (if (Utilities|DoesObjectImplementInterface (.hitactor _outhit) "/Game/Blueprints/Interfaces/BP_Shot.BP_Shot_C")
                    (bind _asbp_phboss (Utilities|Casting|CastToBP_PHBoss (.hitactor _outhit)))
                    (Default|OnShot _asbp_phboss (.hitcomponent _outhit))))
                (:then_1
                  (Utilities|FlowControl|Delay 0.52)
                  (Variables|Default|SetCanFire true))))))))
    (elif (Variables|Default|GetCanFire)
      (Animation|Montage|PlayMontage (Variables|Default|GetFutureArmsMaybe) "/Game/Blueprints/Player/Animations/PH/PHEmptyFire_Montage.PHEmptyFire_Montage"
        (:then
          (Components|Animation|PlayAnimation (Variables|Default|Getgun) "/Game/Objects/Guns/RevolverLukaFinal/Animations/PHRevolverEmptyFire.PHRevolverEmptyFire" false)
          (Utilities|FlowControl|Delay 0.3)
          (Variables|Default|SetCanFire true))))))

(event Input|EnhancedActionEvents|EnhancedInputActionIA_Look
  (params (ActionValue :type Vector%202D%20Structure) (ElapsedSeconds :type Float%20%28double-precision%29) (TriggeredSeconds :type Float%20%28double-precision%29) (InputAction :type Input%20Action%20Object%20Reference :default "/Game/Blueprints/Player/Input/Actions/IA_Look.IA_Look"))
  ;[0.15 0.15 0.15 0.5] The Players Mouse Input
  ;;[0.15 0.15 0.15 0.5 14] Yaw is left to right mouse movement
  (Pawn|Input|AddControllerYawInput (.x ActionValue))
  ;;[0.15 0.15 0.15 0.5 14] Roll is up and down mouse movement
  (Pawn|Input|AddControllerPitchInput (.y ActionValue)))

(event Input|EnhancedActionEvents|EnhancedInputActionIA_Movement
  (params (ActionValue :type Vector%202D%20Structure) (ElapsedSeconds :type Float%20%28double-precision%29) (TriggeredSeconds :type Float%20%28double-precision%29) (InputAction :type Input%20Action%20Object%20Reference :default "/Game/Blueprints/Player/Input/Actions/IA_Movement.IA_Movement"))
  ;[0.15 0.15 0.15 0.5] Movement
  ;;[0.15 0.15 0.15 0.5] Sets Movement for Left and right along actors local Y-Axis
  (Pawn|Input|AddMovementInput (Transformation|GetActorRightVector) (.x ActionValue) false)
  ;;[0.15 0.15 0.15 0.5] Sets Movement for Left and right along actors local X-Axis
  (Pawn|Input|AddMovementInput (Transformation|GetActorForwardVector) (.y ActionValue) false))

(event Input|EnhancedActionEvents|EnhancedInputActionIA_Jump
  (params (ActionValue :type Boolean) (ElapsedSeconds :type Float%20%28double-precision%29) (TriggeredSeconds :type Float%20%28double-precision%29) (InputAction :type Input%20Action%20Object%20Reference :default "/Game/Blueprints/Player/Input/Actions/IA_Jump.IA_Jump"))
  ;[0.15 0.15 0.15 0.5 12] Pretty much self explained outside the fact that stop jumping will let the player know when they can jump again. This can be tweaked a little bit later if we want double jumping and what not
  (:Started
    (Character|Jump))
  (:Completed
    (Character|StopJumping)))

(event Input|EnhancedActionEvents|EnhancedInputActionIA_Reload
  (params (ActionValue :type Boolean) (ElapsedSeconds :type Float%20%28double-precision%29) (TriggeredSeconds :type Float%20%28double-precision%29) (InputAction :type Input%20Action%20Object%20Reference :default "/Game/Blueprints/Player/Input/Actions/IA_Reload.IA_Reload"))
  (if (Variables|Default|GetCanFire)
    (Variables|Default|SetReload true)
    (Variables|Default|SetCanFire false)
    (Animation|Montage|PlayMontage (Variables|Default|GetFutureArmsMaybe) "/Game/Blueprints/Player/Animations/PH/PH_Reload_Montage.PH_Reload_Montage"
      (:then
        (Components|Animation|PlayAnimation (Variables|Default|Getgun) "/Game/Objects/Guns/RevolverLukaFinal/Animations/PH_Reload.PH_Reload" false)
        (Variables|Default|SetBCount 5)
        (Utilities|FlowControl|Delay 1.52)
        (Variables|Default|SetCanFire true)
        (Variables|Default|SetReload false)))))

(event Input|EnhancedActionEvents|EnhancedInputActionIA_ADS
  (params (ActionValue :type Boolean) (ElapsedSeconds :type Float%20%28double-precision%29) (TriggeredSeconds :type Float%20%28double-precision%29) (InputAction :type Input%20Action%20Object%20Reference :default "/Game/Blueprints/Player/Input/Actions/IA_ADS.IA_ADS"))
  (:Ongoing
    (bind _output_get (Variables|Default|SetAiming true))
    (|AimingPrint _output_get)
    (Variables|Default|SetCone%20Half%20Angle%20in%20Degrees 0.0))
  (:Canceled
    (bind _output_get_2 (Variables|Default|SetAiming false))
    (|AimingPrint_2 _output_get_2)
    (Variables|Default|SetCone%20Half%20Angle%20in%20Degrees (Variables|Default|GetAccuracy))))

(event EventBeginPlay
  (bind _revolver_laser (Variables|Default|GetRevolver_Laser))
  (bind _returnvalue (UserInterface|CreateWidget "/Game/UI/W_Main.W_Main_C"))
  (UserInterface|Viewport|AddtoViewport _returnvalue 0)
  (Transformation|AttachComponentToComponent (Variables|Default|Getgun) (Variables|Default|GetFutureArmsMaybe) "Gun" "KeepWorld" "KeepWorld" "KeepWorld" true)
  (Utilities|FlowControl|Sequence
    (:then_0
      (if (Variables|Default|GetLaser)
        (Variables|Default|SetCone%20Half%20Angle%20in%20Degrees 0.0)
        (Variables|Default|SetAccuracy 0.0)
        (Components|StaticMesh|SetStaticMesh _revolver_laser "/Game/Objects/Guns/RevolverLukaFinal/Models/Revolver_Laser.Revolver_Laser")
        (Transformation|AttachComponentToComponent _revolver_laser (Variables|Default|Getgun) "Laser" "SnapToTarget" "SnapToTarget" "SnapToTarget" true)
        (else
          (Variables|Default|SetAccuracy (Variables|Default|GetAccuracy)))))))

(event Collision|EventActorBeginOverlap
  (params (OtherActor :type Actor%20Object%20Reference)))

(event EventTick
  (params (DeltaSeconds :type Float%20%28single-precision%29)))

(event EventControllerChanged
  (params (OldController :type Controller%20Object%20Reference) (NewController :type Controller%20Object%20Reference))
  ;[0.15 0.15 0.15 0.5] Sets up input Mapping Context
  (bind _asbp_player_controller (Utilities|Casting|CastToBP_PlayerController NewController))
  (Input|AddMappingContext (PlayerController|LocalPlayerSubsystems|GetEnhancedInputLocalPlayerSubsystem _asbp_player_controller) "/Game/Blueprints/Player/Input/IMC_PlayerMovement.IMC_PlayerMovement" 0 "(bIgnoreAllPressedKeysUntilRelease=True,bForceImmediately=False,bNotifyUserSettings=False)")
  (Input|AddMappingContext (PlayerController|LocalPlayerSubsystems|GetEnhancedInputLocalPlayerSubsystem _asbp_player_controller) "/Game/Blueprints/Player/Input/IMC_Guns.IMC_Guns" 0 "(bIgnoreAllPressedKeysUntilRelease=True,bForceImmediately=False,bNotifyUserSettings=False)"))

(event Input|KeyboardEvents|X
  (params (Key :type Key%20Structure :default "None"))
  ;[0.15 0.15 0.15 0.5] Health Debug Buttons
  (:Pressed
    (Default|TakeDamage (Variables|Default|GetHealth) 2e+01)))

(event Input|KeyboardEvents|C
  (params (Key :type Key%20Structure :default "None"))
  ;[0.15 0.15 0.15 0.5] Health Debug Buttons
  (:Pressed
    (Default|Heal (Variables|Default|GetHealth) 2e+01)))

(fn ConstructionScript)