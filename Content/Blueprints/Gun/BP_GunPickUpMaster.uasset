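; BP_GunPickUpMaster is a revolver pickup that shows a configured gun and hands it to the player on touch.
; On BeginPlay it snaps the laser, stock and foregrip to sockets named after each component, then applies meshes and skin from GunInfo, with laser taking priority over foregrip.
; When the player character overlaps the sphere, it copies GunInfo to BP_Player, runs SetupGunStats, destroys itself and resets BCount.
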(event OnComponentBeginOverlap(Sphere)
  (params (OverlappedComponent :type Primitive%20Component%20Object%20Reference) (OtherActor :type Actor%20Object%20Reference) (OtherComp :type Primitive%20Component%20Object%20Reference) (OtherBodyIndex :type Integer) (bFromSweep :type Boolean) (SweepResult :type Hit%20Result%20Structure%20%28by%20ref%29))
  (bind _returnvalue (Game|GetPlayerCharacter 0))
  (if (== OtherActor _returnvalue)
    (bind _asbp_player (Utilities|Casting|CastToBP_Player _returnvalue))
    (Variables|/Game/Blueprints/Player/BP_Player.BP_Player_C|SetGunSetup _asbp_player (Variables|Default|GetGunInfo))
    (Default|SetupGunStats _asbp_player)
    (Actor|DestroyActor)
    (Variables|/Game/Blueprints/Player/BP_Player.BP_Player_C|SetBCount _asbp_player 5)))

(event EventBeginPlay
  (bind _output_get (Variables|Default|SetGunParts (Utilities|Array|MakeArray (Variables|Default|GetLaser) (Variables|Default|GetStock) (Variables|Default|GetForegrip))))
  (|Snapsallpartstosockets _output_get
    (:Completed
      (|SetsTheGunApperance))))

(event Collision|EventActorBeginOverlap
  (params (OtherActor :type Actor%20Object%20Reference)))

(event EventTick
  (params (DeltaSeconds :type Float%20%28single-precision%29)))

(fn ConstructionScript)